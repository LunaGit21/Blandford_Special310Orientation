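; NPC Blueprint in the Guard character folder that shows successive dialogue lines on screen when interacted with.
; Each Interact event increments DialogueIndex before reading the Dialogue array, using an inclusive check against the array length.
; The dialogue widget is created for the first player controller and added to the viewport when none exists, then reused for later lines.
; Nothing here resets the index or removes the widget.
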(event EventBeginPlay)

(event Collision|EventActorBeginOverlap
  (params (OtherActor :type Actor%20Object%20Reference)))

(event EventTick
  (params (DeltaSeconds :type Float%20%28single-precision%29)))

(event EventInteract
  (Math|Integer|IncrementInt (Variables|Default|GetDialogueIndex)
    (:%20%20
      (if (<= (Variables|Default|GetDialogueIndex) (Utilities|Array|Length (Variables|Default|GetDialogue)))
        (Variables|Default|GetUI
          (:then
            _)
          (:else
            (bind _returnvalue (UserInterface|CreateWidget "/Game/Blueprints/Interface/WD_Dialgoue.WD_Dialgoue_C" (Game|GetPlayerController 0)))
            (bind _output_get (Variables|Default|SetUI _returnvalue))
            (UserInterface|Viewport|AddtoViewport _output_get 0)))
        (Rendering|Components|TextRender|SetText (Variables|/Game/Blueprints/Interface/WD_Dialgoue.WD_Dialgoue_C|GetDialogueText (Variables|Default|GetUI)) (Utilities|Text|ToText(String) (Utilities|Array|Get(acopy) (Variables|Default|GetDialogue) (Variables|Default|GetDialogueIndex))))))))

(fn ConstructionScript)